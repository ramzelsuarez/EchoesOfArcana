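; BP_NPCSpecial is an always-interactable field NPC that runs a special conversation and can lead into a battle.
; Interacting passes itself and its dialogue row to the game mode.
; AfterSpecialDialogueFinished, if StartsBattle is set, flags a pending Chimkin battle on GI_Core with its area data, stores the player's position, then has GM_Field enter the battle area.
; It reports its own speaker name but a placeholder "None" ID.
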(event `/Game/Definitions/Interfaces/BPI_Interactable.I_Interact`
  (message `/Game/Definitions/Interfaces/BPI_DialogueControl.I_StartSpecialConversation` (`GameplayStatics.GetGameMode`) self (`self.DialogueRow`)))

(event `AfterSpecialDialogueFinished`
  (if (`self.StartsBattle`)
    (bind _asgi_core (cast `/Game/Blueprints/Framework/GI_Core` (`GameplayStatics.GetGameInstance`)))
    (set `/Game/Blueprints/Framework/GI_Core.PendingChimkinBattle` true _asgi_core)
    (`KismetSystemLibrary.PrintString` "PENDING CHIMKIN TRUE")
    (set `/Game/Blueprints/Framework/GI_Core.PendingBattleAreaData` (`self.BattleAreaData`) _asgi_core)
    (bind _asgm_field (cast `/Game/Blueprints/Framework/GM_Field` (`GameplayStatics.GetGameMode`)))
    (message `/Game/Definitions/Interfaces/BPI_InstanceStorage.I_StoreFieldPosition` (`GameplayStatics.GetGameInstance`) (`self.GetTransform` (`GameplayStatics.GetPlayerCharacter` 0)))
    (set `/Game/Blueprints/Framework/GM_Field.CurrentAreaData` (`self.BattleAreaData`) _asgm_field)
    (`/Game/Blueprints/Framework/GM_Field.EnterBattleArea` _asgm_field)))

(fn `I_CanInteract`
  (returns (CanInteract :type Boolean))
  (return true))

(fn `I_GetID`
  (returns (ID :type Name))
  (return "None"))

(fn `I_GetSpeakerName`
  (returns (SpeakerName :type Text))
  (return (`self.SpecialCharName`)))

(fn `UserConstructionScript`)