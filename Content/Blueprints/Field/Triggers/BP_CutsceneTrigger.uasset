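; Field trigger that plays a Level Sequence cutscene once, either when the field player enters its box or, with PlayOnLoad, when the game mode spawns the player.
; It records its trigger through ACIdentifier, binds "player" sequence bindings to the player pawn, and holds cinematic mode until playback ends, then destroys itself.
; Its ID is the sequence's display name, so names must be unique; forced interaction destroys it without playing.
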(event `self.ReceiveBeginPlay`
  (if (`self.PlayOnLoad`)
    (bind _asgm_field (cast `/Game/Blueprints/Framework/GM_Field` (`GameplayStatics.GetGameMode`)))
    (add `/Game/Blueprints/Framework/GM_Field.SpawnedPlayer` _asgm_field (delegate `OnSpawnedPkayer`))))

(event `OnSpawnedPkayer`
  (`self.ForcePlay`))

(event `ForcePlay`
  (`/Engine/EditorBlueprintResources/StandardMacros.DoOnce` false :!label _label
    (:`Completed`
      (`/Game/Blueprints/Components/AC_Identifier.TriggerID` (`self.AC_Identifier`))
      (bind _outactor (`LevelSequencePlayer.CreateLevelSequencePlayer` (`self.LevelSequence`)))
      (`self.TryBindPlayer` _outactor)
      (bind _sequenceplayer (`LevelSequenceActor.SequencePlayer` _outactor))
      (`MovieSceneSequencePlayer.Play` _sequenceplayer)
      (add `MovieSceneSequencePlayer.OnFinished` _sequenceplayer (delegate `OnFinished`))
      (`PlayerController.SetCinematicMode` (`GameplayStatics.GetPlayerController` 0) true false false true true))))

(event `self.Box.OnComponentBeginOverlap`
  (params (OverlappedComponent :type "PrimitiveComponent Object Reference") (OtherActor :type "Actor Object Reference") (OtherComp :type "PrimitiveComponent Object Reference") (OtherBodyIndex :type Integer) (bFromSweep :type Boolean) (SweepResult :type "HitResult Structure (by ref)"))
  (`KismetSystemLibrary.IsObjectOfSoftClass` OtherActor "/Game/Blueprints/Field/BP_FieldPlayer.BP_FieldPlayer_C"
    (:`True`
      (goto _label))))

(event `OnFinished`
  (`PlayerController.SetCinematicMode` (`GameplayStatics.GetPlayerController` 0) false false false true true)
  (`self.K2_DestroyActor`))

(event `/Game/Definitions/Interfaces/BPI_Interactable.I_ForceInteract`
  (`self.K2_DestroyActor`))

(fn `I_CanInteract`
  (returns (CanInteract :type Boolean))
  (return false))

(fn `I_GetID`
  (returns (ID :type Name))
  ; !!: Make sure level sequence names don't overlap
  (return (`KismetStringLibrary.Conv_StringToName` (`KismetSystemLibrary.GetDisplayName` (`self.LevelSequence`)))))

(fn `TryBindPlayer`
  (params (Sequence :type "LevelSequenceActor Object Reference"))
  (for _array_element (`LevelSequenceActor.FindNamedBindings` (`local.Sequence`) "player")
    (`LevelSequenceActor.SetBinding` (`local.Sequence`) _array_element (`|MakeArray` (`GameplayStatics.GetPlayerPawn` 0) :!type "Actor Object Reference") false)))

(fn `UserConstructionScript`)