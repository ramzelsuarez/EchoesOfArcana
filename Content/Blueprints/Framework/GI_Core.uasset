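; Core Game Instance that holds RPG state across levels: party members, their index-matched battle states, inventory, triggered IDs, quest state and field position.
; On Init it seeds party HP/MP, then caches a loaded or new save object for each slot.
; Other systems read and modify this state through interface calls.
; Saving copies state and the pawn's current position to a slot; loading restores the cached copy and opens its saved level.
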(event `self.ReceiveInit`
  (for _array_element (`self.PartyMembers`)
    (bind (_maxhp _maxmp) (break `/Game/Definitions/Structs/S_CharAttributes` (`/Game/Data/DataAssets/BattleCharData/PDA_BattleCharData.InitialAttributes` (`/Game/Data/DataAssets/PartyMemberData/PDA_PartyMemberData.BattleCharData` _array_element))))
    (`KismetArrayLibrary.Array_Add` (`self.PartyStates`) (make `/Game/Definitions/Structs/S_CharState` _maxhp _maxmp 1)))
  (for _index (range (`/Game/Data/DataAssets/GlobalVariables/PDA_GlobalVariables.MaxSaveSlots` (`/Game/Definitions/FunctionLibraries/BPFL_CORE.GetGlobalVariables`)))
    (bind _returnvalue (`KismetStringLibrary.Conv_IntToString` _index))
    (bind _returnvalue_2 (`GameplayStatics.DoesSaveGameExist` _returnvalue))
    (if _returnvalue_2
      (bind _returnvalue_3 (`GameplayStatics.LoadGameFromSlot` _returnvalue))
      (bind _asbp_save_game (cast `/Game/Blueprints/SaveLoad/BP_SaveGame` _returnvalue_3))
      (`KismetArrayLibrary.Array_Add` (`self.SaveGames`) _asbp_save_game)
      (else
        (bind _returnvalue_4 (`GameplayStatics.CreateSaveGameObject` "/Game/Blueprints/SaveLoad/BP_SaveGame.BP_SaveGame_C"))
        (`KismetArrayLibrary.Array_Add` (`self.SaveGames`) _returnvalue_4)))))

(event `/Game/Definitions/Interfaces/BPI_InstanceStorage.I_StoreFieldPosition`
  (params (LastFieldTransform :type "Transform Structure"))
  (`self.StoreFieldPosition` LastFieldTransform))

(event `/Game/Definitions/Interfaces/BPI_InstanceStorage.I_StorePartyStates`
  (params (PartyMembers :type "Array of /Game/Blueprints/Battle/BattleChars/BP_BattleChar_BASE Object Reference (by ref)"))
  (`self.StorePartyStates` PartyMembers))

(event `/Game/Definitions/Interfaces/BPI_InstanceStorage.I_AddItemToInventory`
  (params (ItemData :type "/Game/Data/DataAssets/ItemData/PDA_ItemData Object Reference") (Amount :type Integer))
  (`self.AddItemToInventory` ItemData Amount))

(event `/Game/Definitions/Interfaces/BPI_InstanceStorage.I_AddTriggeredID`
  (params (ID :type Name))
  (`self.AddTriggeredID` ID))

(event `/Game/Definitions/Interfaces/BPI_InstanceStorage.I_SaveGameData`
  (params (SlotIndex :type Integer))
  (`self.SaveGameData` SlotIndex))

(event `/Game/Definitions/Interfaces/BPI_InstanceStorage.I_LoadSaveStateFromSlot`
  (params (SlotIndex :type Integer))
  (`self.LoadGameStateFromSlot` SlotIndex))

(event `/Game/Definitions/Interfaces/BPI_InstanceStorage.I_AddPartyMember`
  (params (NewMember :type "/Game/Data/DataAssets/PartyMemberData/PDA_PartyMemberData Object Reference"))
  (`self.AddPartyMember` NewMember))

(fn `AddItemToInventory`
  (params (ItemData :type "/Game/Data/DataAssets/ItemData/PDA_ItemData Object Reference") (Amount :type Integer))
  (locals (NewAmount :type Integer))
  (set `local.NewAmount` (`KismetMathLibrary.Min` (+ (`BlueprintMapLibrary.Map_Find` (`self.Inventory`) (`local.ItemData`)) (`local.Amount`)) (`/Game/Data/DataAssets/ItemData/PDA_ItemData.MaxStackSize` (`local.ItemData`))))
  (`BlueprintMapLibrary.Map_Add` (`self.Inventory`) (`local.ItemData`) (`local.NewAmount`)))

(fn `AddPartyMember`
  (params (NewMember :type "/Game/Data/DataAssets/PartyMemberData/PDA_PartyMemberData Object Reference"))
  (bind (_maxhp _maxmp) (break `/Game/Definitions/Structs/S_CharAttributes` (`/Game/Data/DataAssets/BattleCharData/PDA_BattleCharData.InitialAttributes` (`/Game/Data/DataAssets/PartyMemberData/PDA_PartyMemberData.BattleCharData` (`local.NewMember`)))))
  (`KismetArrayLibrary.Array_AddUnique` (`self.PartyMembers`) (`local.NewMember`))
  (`KismetArrayLibrary.Array_Add` (`self.PartyStates`) (make `/Game/Definitions/Structs/S_CharState` _maxhp _maxmp 1)))

(fn `AddTriggeredID`
  (params (ID :type "Name (by ref)"))
  (`BlueprintMapLibrary.Map_Add` (`self.TriggeredIDs`) ID true))

(fn `GetAlivePartyMembers`
  (returns (AliveMembers :type "Array of /Game/Data/DataAssets/PartyMemberData/PDA_PartyMemberData Object Reference"))
  (locals (Members :type "Array of /Game/Data/DataAssets/PartyMemberData/PDA_PartyMemberData Object Reference"))
  (for (_array_element _array_index) (`self.PartyStates`)
    (if (not (`.IsKnockedOut_14_79D64E03441BDE08E6B41AAA1ED458F3` (break `/Game/Definitions/Structs/S_CharState` _array_element)))
      (`KismetArrayLibrary.Array_Add` (`local.Members`) (`|GetArrayItem` (`self.PartyMembers`) _array_index))))
  (return (`local.Members`)))

(fn `I_GetAlivePartyMembers`
  (returns (AliveMembers :type "Array of /Game/Data/DataAssets/PartyMemberData/PDA_PartyMemberData Object Reference"))
  (bind _alivemembers (`self.GetAlivePartyMembers`))
  (return _alivemembers))

(fn `I_GetGlobalVariables`
  (returns (GlobalVriables :type "/Game/Data/DataAssets/GlobalVariables/PDA_GlobalVariables Object Reference"))
  (return (`self.GlobalVariables`)))

(fn `I_GetInventory`
  (returns (Inventory :type "Map of /Game/Data/DataAssets/ItemData/PDA_ItemData Object Reference to Integer"))
  (return (`self.Inventory`)))

(fn `I_GetPartyMembers`
  (returns (PartyMembers :type "Array of /Game/Data/DataAssets/PartyMemberData/PDA_PartyMemberData Object Reference"))
  (return (`self.PartyMembers`)))

(fn `I_GetPartyStates`
  (returns (States :type "Array of /Game/Definitions/Structs/S_CharState Structure"))
  (return (`self.PartyStates`)))

(fn `I_GetPlayerFieldPosition`
  (returns (PlayerFieldPosition :type "/Game/Definitions/Structs/S_FieldPosition Structure"))
  (return (`self.PlayerFieldPosition`)))

(fn `I_GetSaveGames`
  (returns (SaveGames :type "Array of /Game/Blueprints/SaveLoad/BP_SaveGame Object Reference"))
  (return (`self.SaveGames`)))

(fn `I_IsIDTriggered`
  (params (ID :type Name))
  (returns (Value :type Boolean))
  (bind _returnvalue (`self.IsIDTriggered` ID))
  (return _returnvalue))

(fn `I_IsSaveDataValid`
  (params (SlotIndex :type Integer))
  (returns (IsValid :type Boolean))
  (bind _returnvalue (`self.IsSaveDataValid` SlotIndex))
  (return _returnvalue))

(fn `I_UseItemFromInventory`
  (params (ItemData :type "/Game/Data/DataAssets/ItemData/PDA_ItemData Object Reference"))
  (returns (FinalAmount :type Integer))
  (bind _finalamount (`self.UseItemFromInventory` ItemData))
  (return _finalamount))

(fn `IsIDTriggered`
  (params (ID :type "Name (by ref)"))
  (returns (ReturnValue :type Boolean))
  (return (`.ReturnValue` (`BlueprintMapLibrary.Map_Find` (`self.TriggeredIDs`) ID))))

(fn `IsSaveDataValid`
  (params (SlotIndex :type Integer))
  (returns (ReturnValue :type Boolean))
  (bind _returnvalue (`GameplayStatics.DoesSaveGameExist` (`KismetStringLibrary.Conv_IntToString` SlotIndex)))
  (return _returnvalue))

(fn `LoadGameStateFromSlot`
  (params (SlotIndex :type Integer))
  (locals (SaveGame :type "/Game/Blueprints/SaveLoad/BP_SaveGame Object Reference"))
  (set `local.SaveGame` (`|GetArrayItem` (`self.SaveGames`) (`local.SlotIndex`)))
  (`|ExecutionSequence`
    (:`then_0`
      ; Apply values to GameInstance
      (set `self.PartyMembers` (`/Game/Blueprints/SaveLoad/BP_SaveGame.PartyMembers` (`local.SaveGame`))))
    (:`then_1`
      (set `self.PlayerFieldPosition` (`/Game/Blueprints/SaveLoad/BP_SaveGame.PlayerFieldPosition` (`local.SaveGame`))))
    (:`then_2`
      (set `self.PartyStates` (`/Game/Blueprints/SaveLoad/BP_SaveGame.PartyStates` (`local.SaveGame`))))
    (:`then_3`
      (set `self.Inventory` (`/Game/Blueprints/SaveLoad/BP_SaveGame.Inventory` (`local.SaveGame`))))
    (:`then_4`
      (set `self.TriggeredIDs` (`/Game/Blueprints/SaveLoad/BP_SaveGame.TriggeredIDs` (`local.SaveGame`))))
    (:`then_5`
      (set `self.ChimkinQuestState` (`/Game/Blueprints/SaveLoad/BP_SaveGame.ChimkinQuestState` (`local.SaveGame`))))
    (:`then_6`
      ; Actually load the stage
      (`GameplayStatics.OpenLevel` (`KismetStringLibrary.Conv_StringToName` (`.FieldLevelName_2_4EFACB7A41468F38A405899DDEDB5CE3` (break `/Game/Definitions/Structs/S_FieldPosition` (`/Game/Blueprints/SaveLoad/BP_SaveGame.PlayerFieldPosition` (`local.SaveGame`)))))))))

(fn `SaveGameData`
  (params (SlotIndex :type Integer))
  (locals (SaveGame :type "/Game/Blueprints/SaveLoad/BP_SaveGame Object Reference"))
  (set `local.SaveGame` (`|GetArrayItem` (`self.SaveGames`) (`local.SlotIndex`)))
  (set `/Game/Blueprints/SaveLoad/BP_SaveGame.PartyMembers` (`self.PartyMembers`) (`local.SaveGame`))
  (set `/Game/Blueprints/SaveLoad/BP_SaveGame.Inventory` (`self.Inventory`) (`local.SaveGame`))
  (set `/Game/Blueprints/SaveLoad/BP_SaveGame.TriggeredIDs` (`self.TriggeredIDs`) (`local.SaveGame`))
  (set `/Game/Blueprints/SaveLoad/BP_SaveGame.ChimkinQuestState` (`self.ChimkinQuestState`) (`local.SaveGame`))
  (set `/Game/Blueprints/SaveLoad/BP_SaveGame.PartyStates` (`self.PartyStates`) (`local.SaveGame`))
  (set `/Game/Blueprints/SaveLoad/BP_SaveGame.DateTime` (`KismetMathLibrary.Now`) (`local.SaveGame`))
  (bind _areadata (message `/Game/Definitions/Interfaces/BPI_AreaControl.I_GetCurrentAreaData` (`GameplayStatics.GetGameMode`)))
  (bind _returnvalue (`GameplayStatics.GetCurrentLevelName` true))
  (set `/Game/Blueprints/SaveLoad/BP_SaveGame.PlayerFieldPosition` (make `/Game/Definitions/Structs/S_FieldPosition` _returnvalue (`Actor.GetTransform` (`GameplayStatics.GetPlayerPawn` 0)) _areadata) (`local.SaveGame`))
  (`GameplayStatics.SaveGameToSlot` (`local.SaveGame`) (`KismetStringLibrary.Conv_IntToString` (`local.SlotIndex`)))
  (`self.SavedGame`))

(fn `StoreFieldPosition`
  (params (LastFieldTransform :type "Transform Structure"))
  (setmembers `/Game/Definitions/Structs/S_FieldPosition` :`StructRef` (`self.PlayerFieldPosition`) :`LastFieldTransform` LastFieldTransform)
  (bind _areadata (message `/Game/Definitions/Interfaces/BPI_AreaControl.I_GetCurrentAreaData` (`GameplayStatics.GetGameMode`)))
  (bind _returnvalue (`GameplayStatics.GetCurrentLevelName` true))
  (setmembers `/Game/Definitions/Structs/S_FieldPosition` :`StructRef` (`self.PlayerFieldPosition`) :`FieldLevelName` _returnvalue :`AreaInfo` _areadata))

(fn `StorePartyStates`
  (params (PartyMembers :type "Array of /Game/Blueprints/Battle/BattleChars/BP_BattleChar_BASE Object Reference"))
  (for (_array_element _array_index) PartyMembers
    (`KismetArrayLibrary.Array_Set` (`self.PartyStates`) _array_index (`/Game/Blueprints/Components/AC_BattleStats.State` (`/Game/Blueprints/Battle/BattleChars/BP_BattleChar_BASE.AC_BattleStats` _array_element)) true)))

(fn `UseItemFromInventory`
  (params (ItemData :type "/Game/Data/DataAssets/ItemData/PDA_ItemData Object Reference"))
  (returns (FinalAmount :type Integer))
  (locals (NewAmount :type Integer))
  (set `local.NewAmount` (- (`BlueprintMapLibrary.Map_Find` (`self.Inventory`) (`local.ItemData`)) 1))
  (if (<= (`local.NewAmount`) 0)
    (`BlueprintMapLibrary.Map_Remove` (`self.Inventory`) (`local.ItemData`))
    (else
      (`BlueprintMapLibrary.Map_Add` (`self.Inventory`) (`local.ItemData`) (`local.NewAmount`))))
  (return (`local.NewAmount`)))