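; PC_Core is the core player controller, owning the field and battle HUD widgets and switching UI input modes.
; Interface events create those widgets, toggle cursor and input mode between game-and-UI and game-only, and remove the field input mapping context.
; Interface getters expose the stored widgets to other Blueprints.
; Debug keys toggle fast-forward through global time dilation and open the load screen with UI controls active.
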(event EventBeginPlay)

(event EventTick
  (params (DeltaSeconds :type Float%20%28single-precision%29)))

(event Input|KeyboardEvents|DebugKeyL
  (params (Key :type Key%20Structure :default "None") (ActionValue :type Input%20Action%20Value%20Structure))
  (:Pressed
    (bind _returnvalue (UserInterface|CreateWidget "/Game/UI/Widgets/SaveLoad/WBP_LoadScreen.WBP_LoadScreen_C" 0 (Variables|Default|GetMainMenuWidget)))
    (UserInterface|Viewport|AddtoViewport _returnvalue 0)
    (CallFunction|ActivateUIControls _returnvalue)))

(event Input|KeyboardEvents|Q
  (params (Key :type Key%20Structure :default "None"))
  (:Pressed
    (bind _isa (Utilities|FlowControl|FlipFlop)
      (:A
        _)
      (:B
        _))
    (Utilities|Time|SetGlobalTimeDilation (Math|Float|SelectFloat 3.0 1.0 _isa))))

(event EventIInitWidgetBattle
  (CallFunction|InitWidgetBattle))

(event EventIInitWidgetField
  (CallFunction|InitWidgetField))

(event EventIDisableFieldInputs
  (CallFunction|DisableFieldInputs))

(event EventIActivateUIControls
  (params (WidgetToFocus :type Widget%20Object%20Reference))
  (CallFunction|ActivateUIControls WidgetToFocus))

(event EventIDeactivateUIControls
  (CallFunction|DeactivateUIControls))

(fn ConstructionScript)

(fn InitWidgetBattle
  (bind _returnvalue (UserInterface|CreateWidget "/Game/UI/Widgets/WBP_Battle.WBP_Battle_C" self))
  (bind _output_get (Variables|Default|SetWidgetBattle _returnvalue))
  (UserInterface|Viewport|AddtoViewport _output_get 0))

(fn InitWidgetField
  (bind _returnvalue (UserInterface|CreateWidget "/Game/UI/Widgets/WBP_Field.WBP_Field_C" self 0))
  (bind _output_get (Variables|Default|SetWidgetField _returnvalue))
  (UserInterface|Viewport|AddtoViewport _output_get 0))

(fn ActivateUIControls
  (params (InWidgetToFocus :type Widget%20Object%20Reference))
  (Input|SetInputModeGameandUI (Game|GetPlayerController 0) InWidgetToFocus "DoNotLock" true true)
  (Variables|/Script/Engine.PlayerController|SetbShowMouseCursor (Game|GetPlayerController 0) true))

(fn DeactivateUIControls
  (Input|SetInputModeGameOnly (Game|GetPlayerController 0) true)
  (Variables|/Script/Engine.PlayerController|SetbShowMouseCursor (Game|GetPlayerController 0) false))

(fn DisableFieldInputs
  (Input|RemoveMappingContext (PlayerController|LocalPlayerSubsystems|GetEnhancedInputLocalPlayerSubsystem self) "/Game/Inputs/Field/IMC_Field.IMC_Field" "(bIgnoreAllPressedKeysUntilRelease=True,bForceImmediately=False,bNotifyUserSettings=False)"))

(fn IGetWidgetBattle
  (return (Variables|Default|GetWidgetBattle)))

(fn IGetWidgetField
  (return (Variables|Default|GetWidgetField)))