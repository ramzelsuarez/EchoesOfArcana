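; Turn-based battle manager pawn that spawns warrior party and slime enemy teams, gets possessed by the player controller and sways its camera with a timeline.
; Turns cycle party first, then enemies, refilling the order and turn-order widget when empty.
; Party members slide to an active spot and back via timelines; enemies just wait, with no combat actions yet.
; ConcludeBattle reloads the saved field level, but its only caller is disconnected.
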(event `self.ReceiveBeginPlay`
  (message `/Game/Definitions/Interfaces/BPI_UIControl.I_InitWidgetBattle` (`GameplayStatics.GetPlayerController` 0))
  (`self.StartBattle`))

(event `StartCameraSway`
  (bind (_relativerotation_roll _relativerotation_pitch) (`KismetMathLibrary.BreakRotator` (`SceneComponent.RelativeRotation` (`self.Camera`))))
  (`TimelineComponent.SetPlayRate` (`self.AnimCameraSway`) (`self.CameraSwayRate`))
  (bind (_direction _yawrotation) (`Timeline|AnimCameraSway`)
    (:`Update`
      (`SceneComponent.K2_SetRelativeRotation` (`self.Camera`) (`KismetMathLibrary.MakeRotator` _relativerotation_roll _relativerotation_pitch (* _yawrotation (`self.CameraSwayDistance`))) false false))))

(event `StartBattle`
  (for _array_element (`self.EnemyTeamLocations`)
    (bind _returnvalue (`|SpawnActorFromClass` "/Game/Blueprints/Battle/BattleChars/Enemies/Slime/BP_BattleSlime.BP_BattleSlime_C" (`KismetMathLibrary.MakeTransform` (+ _array_element (`self.SpawnHeightOffset`) (`self.K2_GetActorLocation`))) "AlwaysSpawn" "MultiplyWithRoot" null null))
    (`KismetArrayLibrary.Array_AddUnique` (`self.EnemyTeam`) _returnvalue))
  (for _array_element_2 (`self.PartyTeamLocations`)
    (bind _returnvalue_2 (`|SpawnActorFromClass` "/Game/Blueprints/Battle/BattleChars/Party/Warrior/BP_BattleWarrior.BP_BattleWarrior_C" (`KismetMathLibrary.MakeTransform` (+ _array_element_2 (`self.SpawnHeightOffset`) (`self.K2_GetActorLocation`)) (`self.PartyTeamRotation`)) "AlwaysSpawn" "MultiplyWithRoot" null null))
    (`KismetArrayLibrary.Array_AddUnique` (`self.PartyTeam`) _returnvalue_2))
  (`self.DecideTurnOrder`)
  (`self.SelectActiveCharacter`)
  (`self.StartCameraSway`)
  (`Controller.Possess` (`GameplayStatics.GetPlayerController` 0) self)
  (`self.StartTurn`))

(event `ConcludeBattle`
  (bind _playerfieldposition (message `/Game/Definitions/Interfaces/BPI_InstanceStorage.I_GetPlayerFieldPosition` (`GameplayStatics.GetGameInstance`)))
  (`GameplayStatics.OpenLevel` (`KismetStringLibrary.Conv_StringToName` (`.FieldLevelName_2_4EFACB7A41468F38A405899DDEDB5CE3` (break `/Game/Definitions/Structs/S_FieldPosition` _playerfieldposition)))))

(event `StartTurn`
  (`KismetSystemLibrary.PrintString` (`KismetStringLibrary.Concat_StrStr` (`KismetSystemLibrary.GetDisplayName` (`self.ActiveCharacter`)) "is Active!"))
  (if (`/Game/Blueprints/Battle/BattleChars/BP_BattleChar_BASE.IsPartyMember` (`self.ActiveCharacter`))
    (`self.MoveToActive`)
    (else
      (`KismetSystemLibrary.Delay` 2.0)
      (`self.ConcludeTurn`))))

(event `MoveToActive`
  ;[0.15 0.1362 0.01071 0.5] Move To Active
  (`TimelineComponent.SetPlayRate` (`self.AnimMoveToActive`) 2.0) ; TODO: Get rid of magic number
  (bind (_direction _alpha) (`Timeline|AnimMoveToActive` :!via `PlayFromStart`)
    (:`Update`
      (`self.K2_SetActorLocation` (`self.ActiveCharacter`) (`KismetMathLibrary.VLerp` (`/Game/Blueprints/Battle/BattleChars/BP_BattleChar_BASE.SpawnedLocation` (`self.ActiveCharacter`)) (`self.AdjustedActiveLocation`) _alpha) false false))
    (:`Finished`
      (`KismetSystemLibrary.Delay` 2.0)
      (`self.MoveBackFromActive`))))

(event `MoveBackFromActive`
  ;[0.15 0.1362 0.01071 0.5] Move Back From Active
  (`TimelineComponent.SetPlayRate` (`self.AnimMoveBackFromActive`) 2.0) ; TODO: Get rid of magic number
  (bind (_direction _alpha) (`Timeline|AnimMoveBackFromActive` :!via `PlayFromStart`)
    (:`Update`
      (`self.K2_SetActorLocation` (`self.ActiveCharacter`) (`KismetMathLibrary.VLerp` (`self.AdjustedActiveLocation`) (`/Game/Blueprints/Battle/BattleChars/BP_BattleChar_BASE.SpawnedLocation` (`self.ActiveCharacter`)) _alpha) false false))
    (:`Finished`
      (`KismetSystemLibrary.Delay` 1.0)
      (`self.ConcludeTurn`))))

(event `ConcludeTurn`
  (`/Game/Blueprints/Battle/BattleChars/BP_BattleChar_BASE.HideBattlePortrait` (`self.ActiveCharacter`))
  (`KismetArrayLibrary.Array_Remove` (`self.TurnOrder`))
  (if (`KismetArrayLibrary.Array_IsEmpty` (`self.TurnOrder`))
    (`self.DecideTurnOrder`)
    (`self.SelectActiveCharacter`)
    (`self.StartTurn`)
    (else
      (`self.SelectActiveCharacter`)
      (`self.StartTurn`))))

(fn `DecideTurnOrder`
  (`KismetArrayLibrary.Array_Clear` (`self.TurnOrder`))
  (`KismetArrayLibrary.Array_Append` (`self.TurnOrder`) (`self.PartyTeam`))
  (`KismetArrayLibrary.Array_Append` (`self.TurnOrder`) (`self.EnemyTeam`))
  (bind _widgetbattle (message `/Game/Definitions/Interfaces/BPI_UIControl.I_GetWidgetBattle` (`GameplayStatics.GetPlayerController` 0)))
  (`/Game/UI/Widgets/Battle/WBP_TurnOrder.ReplaceTurnOrder` (`/Game/UI/Widgets/WBP_Battle.WBP_TurnOrder` _widgetbattle) (`self.TurnOrder`)))

(fn `SelectActiveCharacter`
  (set `self.ActiveCharacter` (`|GetArrayItem` (`self.TurnOrder`))))

(fn `UserConstructionScript`)