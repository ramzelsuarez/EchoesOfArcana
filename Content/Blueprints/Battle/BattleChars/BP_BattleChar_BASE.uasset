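; Base actor for battle characters, handling sprite animation, voice lines, target pointer and other combat widgets.
; Attacks play a skill or default animation override, or a jump timeline without one, and report completion to BattleManager.
; Received skills spawn particles and route damage or healing to ACBattleStats by target group.
; On depleted health, BattleManager is updated; party members switch to a downed state, others play a knockout timeline and hide.
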(event `self.ReceiveBeginPlay`
  (`|ExecutionSequence`
    (:`then_0`
      (set `self.SpawnedLocation` (`self.K2_GetActorLocation`))
      (bind _aswbp_target_pointer (cast `/Game/UI/Widgets/WBP_TargetPointer` (`WidgetComponent.GetUserWidgetObject` (`self.WidgetPointer`))))
      (set `self.WidgetTargetPointer` _aswbp_target_pointer)
      (bind _aswbp_combat_text (cast `/Game/UI/Widgets/Battle/WBP_CombatText` (`WidgetComponent.GetUserWidgetObject` (`self.WidgetCombatText`))))
      (set `self.WidgetCombatNumber` _aswbp_combat_text))
    (:`then_1`
      (`/Game/Blueprints/Components/AC_Shaker.Initialize` (`self.AC_Shaker`) (`self.Sprite`))
      (`/Game/Blueprints/Components/AC_BattleStats.Initialize` (`self.AC_BattleStats`) self))
    (:`then_2`
      (bind _returnvalue (`PrimitiveComponent.CreateDynamicMaterialInstance` (`self.Sprite`) 0 null "None"))
      (set `self.DynamicSpriteMat` _returnvalue))))

(event `PlayAttackAnim`
  (params (SkillData :type "/Game/Data/DataAssets/SkillData/PDA_SkillData Object Reference"))
  (bind (_spawnedlocation_x _spawnedlocation_y _spawnedlocation_z) (`KismetMathLibrary.BreakVector` (`self.SpawnedLocation`)))
  (bind _animation (`self.PickSkillAnim` SkillData))
  (`/Engine/EditorBlueprintResources/StandardMacros.IsValid` _animation
    (:`Is Valid`
      (`PaperZDPlaySlotOverrideAction.PlayAnimationOverrideWithCallbacks` (`PaperZDAnimationComponent.AnimInstance` (`self.AnimationComponent`)) _animation
        (:`then`
          (`/Game/Blueprints/Components/AC_BattleStats.UpdateMana` (`self.AC_BattleStats`) (* (`/Game/Data/DataAssets/SkillData/PDA_SkillData.ManaCost` SkillData) -1.0)))
        (:`OnCompleted`
          (`KismetSystemLibrary.RetriggerableDelay` (`/Game/Data/DataAssets/GlobalVariables/PDA_GlobalVariables.DelayAfterAttackAnim` (`/Game/Definitions/FunctionLibraries/BPFL_CORE.GetGlobalVariables`)) :!label _label)
          (`/Game/Blueprints/Battle/BP_BattleManager.MoveBackFromActive` (`self.BattleManager`)))
        (:`OnCancelled`
          (goto _label))))
    (:`Is Not Valid`
      (`TimelineComponent.SetPlayRate` (`self.AnimDoubleJump`) (`self.JumpPlayRate`))
      (bind (_direction _alpha) (`Timeline|AnimDoubleJump` :!via `PlayFromStart`)
        (:`Update`
          (`self.K2_SetActorLocation` (`KismetMathLibrary.MakeVector` _spawnedlocation_x _spawnedlocation_y (+ _spawnedlocation_z (* _alpha (`self.JumpHeight`))))))
        (:`Finished`
          (`/Game/Blueprints/Battle/BP_BattleManager.FinishedTimelineAttackAnim` (`self.BattleManager`)))))))

(event `PlayKnockoutAnim`
  (`TimelineComponent.SetPlayRate` (`self.AnimKnockout`) (`self.KnockoutAnimPlayRate`))
  (bind (_direction _alpha) (`Timeline|AnimKnockout` :!via `PlayFromStart`)
    (:`Update`
      (`self.K2_SetActorLocation` (`KismetMathLibrary.VLerp` (`self.SpawnedLocation`) (+ (`self.SpawnedLocation`) (`self.KnockoutOffset`)) _alpha)))
    (:`Finished`
      (`self.SetActorHiddenInGame` true))))

(event `PlayVoiceLine`
  (params (Line :type "/Game/Definitions/Enums/E_VoiceLines Enum" :default "NewEnumerator0"))
  (bind (_value _returnvalue) (`BlueprintMapLibrary.Map_Find` (`/Game/Data/DataAssets/BattleCharData/PDA_BattleCharData.VoiceLines` (`self.BattleCharData`)) Line))
  (if _returnvalue
    (bind _object (`|LoadAsset` _value)
      (:`Completed`
        (bind _assound_cue (cast `SoundCue` _object))
        (`GameplayStatics.PlaySoundAtLocation` _assound_cue (`self.K2_GetActorLocation`) (struct) 1.0 1.0 0.0 null null null null)))))

(fn `AssignBattleHealthManaWidget`
  (params (WidgetHealthMana :type "/Game/UI/Widgets/Battle/WBP_BattleHealthMana Object Reference"))
  (bind (_maxhp _maxmp) (break `/Game/Definitions/Structs/S_CharAttributes` (`/Game/Blueprints/Components/AC_BattleStats.Attributes` (`self.AC_BattleStats`))))
  (bind (_hp _mp) (break `/Game/Definitions/Structs/S_CharState` (`/Game/Blueprints/Components/AC_BattleStats.State` (`self.AC_BattleStats`))))
  (set `self.WidgetHealthMana` WidgetHealthMana)
  (`/Game/UI/Widgets/Battle/WBP_BattleHealthMana.Activate` (`self.WidgetHealthMana`) (`/Game/Data/DataAssets/BattleCharData/PDA_BattleCharData.DisplayName` (`self.BattleCharData`)) _maxhp _hp _maxmp _mp))

(fn `DepletedHealth`
  (`|ExecutionSequence`
    (:`then_0`
      (`/Game/Blueprints/Battle/BP_BattleManager.UpdateTeamAlive` (`self.BattleManager`) self)
      (bind _widgetportrait (`self.WidgetPortrait`)
        (:`then`
          (`/Game/UI/Widgets/Battle/WBP_Portrait.HidePortrait` _widgetportrait))
        (:`else`)))
    (:`then_1`
      (if (`self.IsPartyMember`)
        (`PaperZDAnimInstance.JumpToNode` (`PaperZDAnimationComponent.AnimInstance` (`self.AnimationComponent`)) "JumpDowned" "None")
        (else
          (`self.PlayKnockoutAnim`))))))

(fn `ExecuteBattleEffect`
  (`/Game/Blueprints/Battle/BP_BattleManager.ApplyBattleEffect` (`self.BattleManager`) (`self.AC_BattleStats`)))

(fn `ForceKnockoutAnim`
  (`PaperZDAnimInstance.JumpToNode` (`PaperZDAnimationComponent.AnimInstance` (`self.AnimationComponent`)) "JumpDowned" "None"))

(fn `GetSkillByIndex`
  (params (Index :type Integer))
  (returns (SkillData :type "/Game/Data/DataAssets/SkillData/PDA_SkillData Object Reference"))
  (if (<= Index -1)
    (return (`/Game/Data/DataAssets/BattleCharData/PDA_BattleCharData.BasicAttackData` (`self.BattleCharData`)))
    (else
      (return (`|GetArrayItem` (`/Game/Blueprints/Components/AC_BattleStats.Skills` (`self.AC_BattleStats`)) (`local.Index`))))))

(fn `HideBattlePortrait`
  (bind _widgetportrait (`self.WidgetPortrait`)
    (:`then`
      (`/Game/UI/Widgets/Battle/WBP_Portrait.HidePortrait` _widgetportrait)
      (set `self.WidgetPortrait` null))
    (:`else`)))

(fn `PickSkillAnim`
  (params (SkillData :type "/Game/Data/DataAssets/SkillData/PDA_SkillData Object Reference"))
  (returns (Animation :type "PaperZDAnimSequence Object Reference"))
  (bind _battlechardata (`self.BattleCharData`))
  (`/Engine/EditorBlueprintResources/StandardMacros.IsValid` SkillData
    (:`Is Valid`
      (bind _animation (`/Game/Data/DataAssets/SkillData/PDA_SkillData.Animation` (`local.SkillData`))
        (:`then`
          (return _animation))
        (:`else`
          _)))
    (:`Is Not Valid`
      _))
  (return (select `bool` (`/Game/Data/DataAssets/SkillData/PDA_SkillData.IsItemSkill` (`local.SkillData`)) :`false` (`/Game/Data/DataAssets/BattleCharData/PDA_BattleCharData.AttackAnimDefault` _battlechardata) :`true` (`/Game/Data/DataAssets/BattleCharData/PDA_BattleCharData.ItemAnimDefault` _battlechardata))))

(fn `ReceiveBattleEffect`
  (params (InstigatorStats :type "/Game/Blueprints/Components/AC_BattleStats Object Reference") (SkillData :type "/Game/Data/DataAssets/SkillData/PDA_SkillData Object Reference"))
  (`NiagaraFunctionLibrary.SpawnSystemAtLocation` (`/Game/Data/DataAssets/SkillData/PDA_SkillData.ParticleEffect` (`local.SkillData`)) (`SceneComponent.K2_GetComponentLocation` (select `/Game/Definitions/Enums/E_TargetPosition` (`/Game/Data/DataAssets/SkillData/PDA_SkillData.ParticlePosition` (`local.SkillData`)) :`NewEnumerator0` (`self.Loc_Head`) :`NewEnumerator1` (`self.Loc_Middle`) :`NewEnumerator2` (`self.Loc_Feet`))) (struct :`Yaw` 180.0) (1.0 1.0 1.0) true true "AutoRelease")
  (switch `/Game/Definitions/Enums/E_TargetGroup` (`/Game/Data/DataAssets/SkillData/PDA_SkillData.TargetGroup` (`local.SkillData`))
    (:`NewEnumerator0`
      (`/Game/Blueprints/Components/AC_BattleStats.ReceiveDamageEffect` (`self.AC_BattleStats`) (`local.InstigatorStats`) (`local.SkillData`)))
    (:`NewEnumerator1`
      (`/Game/Blueprints/Components/AC_BattleStats.ReceiveHealEffect` (`self.AC_BattleStats`) (`local.InstigatorStats`) (`local.SkillData`)))))

(fn `SetDefending`
  (params (SetActive :type Boolean))
  (set `self.IsDefending` SetActive))

(fn `SetPointerVisibility`
  (params (SetVisible :type Boolean))
  (if SetVisible
    (`/Game/UI/Widgets/WBP_TargetPointer.ShowPointer` (`self.WidgetTargetPointer`))
    (`MaterialInstanceDynamic.SetScalarParameterValue` (`self.DynamicSpriteMat`) "IsPulsing" 1.0)
    (else
      (`/Game/UI/Widgets/WBP_TargetPointer.HidePointer` (`self.WidgetTargetPointer`))
      (`MaterialInstanceDynamic.SetScalarParameterValue` (`self.DynamicSpriteMat`) "IsPulsing" 0.0))))

(fn `UserConstructionScript`)