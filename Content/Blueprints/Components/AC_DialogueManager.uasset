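; Dialogue manager component that runs linear NPC conversations from rows in DT_Dialogue.
; Each line shows on the player controller's field widget over player or target with a sound cue, then chains through NextRow until none remains.
; Interface messages set conversation locks on player and NPC; special conversations lock only the player.
; Ending clears locks, hides the widget and notifies quest-giver or special NPCs that dialogue finished.
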(fn `EndConversation`
  (message `/Game/Definitions/Interfaces/BPI_DialogueControl.I_SetCoversationLock` (`GameplayStatics.GetPlayerPawn` 0) false)
  (message `/Game/Definitions/Interfaces/BPI_DialogueControl.I_SetCoversationLock` (`self.Target Actor`) false)
  (`self.HideWidget`)
  (bind _asbp_npcquest_giver (cast `/Game/Blueprints/Field/NPCs/BP_NPCQuestGiver` (`self.Target Actor`))
    (:`then`
      (`/Game/Blueprints/Field/NPCs/BP_NPCQuestGiver.AfterQuestDialogueFinished` _asbp_npcquest_giver))
    (:`CastFailed`
      (bind _asbp_npcspecial (cast `/Game/Blueprints/Field/NPCs/BP_NPCSpecial` (`self.Target Actor`)))
      (`/Game/Blueprints/Field/NPCs/BP_NPCSpecial.AfterSpecialDialogueFinished` _asbp_npcspecial))))

(fn `HideWidget`
  (bind _widgetfield (message `/Game/Definitions/Interfaces/BPI_UIControl.I_GetWidgetField` (`GameplayStatics.GetPlayerController` 0)))
  (`/Game/UI/Widgets/WBP_Field.HIdeDialogue` _widgetfield))

(fn `ProcessDialogueLine`
  (params (RowName :type Name) (TargetActor :type "Actor Object Reference"))
  (returns (FoundRow :type Boolean))
  (bind (_message _nextrow _isplayer) (break `/Game/Definitions/Structs/DataTables/S_DialogueData` (`self.CurrentDialogueLine`)))
  (bind _returnvalue (`|GetDataTableRow` "/Game/Data/DataTables/DT_Dialogue.DT_Dialogue" (`local.RowName`))
    (:`then`
      (set `self.CurrentDialogueLine` _returnvalue)
      (set `self.Target Actor` (`local.TargetActor`))
      (bind _widgetfield (message `/Game/Definitions/Interfaces/BPI_UIControl.I_GetWidgetField` (`GameplayStatics.GetPlayerController` 0)))
      (`/Game/UI/Widgets/WBP_Field.ShowDialogue` _widgetfield (select `bool` _isplayer :`false` (`local.TargetActor`) :`true` (`GameplayStatics.GetPlayerPawn` 0) :!type "Actor Object Reference") _message)
      (`GameplayStatics.PlaySound2D` "/Game/Art/Audio/SFX/S_Dialogue_Cue.S_Dialogue_Cue" 1.0 1.0 0.0 null null)
      (return true))
    (:`RowNotFound`
      (return false))))

(fn `ProgressConversation`
  (bind ((`NextRow_5_44B477E14B8A79692F8EDFA431D4B0BE` _nextrow)) (break `/Game/Definitions/Structs/DataTables/S_DialogueData` (`self.CurrentDialogueLine`)))
  (if (== (`.NextRow_5_44B477E14B8A79692F8EDFA431D4B0BE` (break `/Game/Definitions/Structs/DataTables/S_DialogueData` (`self.CurrentDialogueLine`))) "None")
    (`self.EndConversation`)
    (else
      (bind _foundrow (`self.ProcessDialogueLine` _nextrow (`self.Target Actor`)))
      (if (not _foundrow)
        (`KismetSystemLibrary.PrintText` (`|FormatText` "Line Not Found: {Row}" _nextrow) true true (struct :`R` 0.201021 :`G` 0.005452 :`B` 0.016582 :`A` 1.0))
        (`self.EndConversation`)))))

(fn `StartConversation`
  (params (ConversationTarget :type "/Game/Blueprints/Field/NPCs/BP_NPC Object Reference") (RowName :type Name))
  (bind _foundrow (`self.ProcessDialogueLine` (`local.RowName`) (`local.ConversationTarget`)))
  (if _foundrow
    (message `/Game/Definitions/Interfaces/BPI_DialogueControl.I_SetCoversationLock` (`GameplayStatics.GetPlayerPawn` 0) true)
    (message `/Game/Definitions/Interfaces/BPI_DialogueControl.I_SetCoversationLock` (`local.ConversationTarget`) true)))

(fn `StartSpecialConversation`
  (params (SpecialCharaTarget :type "/Game/Blueprints/Field/NPCs/BP_NPCSpecial Object Reference") (RowName :type Name))
  (bind _foundrow (`self.ProcessDialogueLine` (`local.RowName`) (`local.SpecialCharaTarget`)))
  (if _foundrow
    (message `/Game/Definitions/Interfaces/BPI_DialogueControl.I_SetCoversationLock` (`GameplayStatics.GetPlayerPawn` 0) true)
    (message `/Game/Definitions/Interfaces/BPI_DialogueControl.I_SetCoversationLock` (`self.Target Actor`) false)))